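; BP_Character is a character prop with flipbook-style mesh animation, a cutscene reveal and an unfinished dissolve effect.
; PlayAnim starts a FrameRate-driven timer that steps StaticMesh through the Meshes array, clearing itself at the end.
; StartPlayerCutScene makes the mesh visible.
; DissolveCharacter makes Tick decrease DissolveAmount, but the nodes passing it to the dynamic material and NSDissolve "Mask" parameters are disconnected.
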(event Custom|PlayAnim
  (Utilities|Time|SetTimerbyFunctionName 0 "PlayAnimation" (/ 1.0 (Variables|Default|GetFrameRate)) true))

(event Custom|DissolveCharacter
  (Variables|Default|SetDissolve true)
  (Development|PrintText "Hello"))

(event Custom|StartPlayerCutScene
  (Rendering|SetVisibility (Variables|Default|GetStaticMesh) true false))

(event EventBeginPlay
  (bind _returnvalue (Rendering|Material|CreateDynamicMaterialInstance (Variables|Default|GetStaticMesh) 0 0 "None" :!class /Script/Engine.PrimitiveComponent))
  (Variables|Default|SetMaterialInstance _returnvalue))

(event EventTick
  (params (DeltaSeconds :type Float%20%28single-precision%29))
  (if (Variables|Default|GetDissolve)
    (Variables|Default|SetDissolveAmount (* (- (Variables|Default|GetDissolveAmount) DeltaSeconds) 1.0))))

(fn ConstructionScript)

(fn PlayAnimation
  (bind _meshes (Variables|Default|GetMeshes))
  (Variables|Default|SetCurrentIndex (+ (Variables|Default|GetCurrentIndex) 1))
  (if (>= (Variables|Default|GetCurrentIndex) (Utilities|Array|Length _meshes))
    (Variables|Default|SetCurrentIndex 0)
    (Utilities|Time|ClearTimerbyFunctionName 0 "PlayAnimation")
    (else
      (Components|StaticMesh|SetStaticMesh (Variables|Default|GetStaticMesh) (Utilities|Array|Get(acopy) _meshes (Variables|Default|GetCurrentIndex))))))