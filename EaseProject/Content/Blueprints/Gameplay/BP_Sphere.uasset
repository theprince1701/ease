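; Interactable sphere actor that activates the ending event in the main scene, or plays a level sequence in other scenes.
; Activation spawns rocks and shakes the camera, then a delayed chain fires an extraction beam, a sequence, sphere growth and the end widget.
; Tick ramps material, light and color-fill intensity, while random line traces spawn Niagara lightning at surface hits, increasingly often after activation.
; A separate Transition event opens SecondScene.
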(event OnComponentBeginOverlap(Sphere1)
  (params (OverlappedComponent :type Primitive%20Component%20Object%20Reference) (OtherActor :type Actor%20Object%20Reference) (OtherComp :type Primitive%20Component%20Object%20Reference) (OtherBodyIndex :type Integer) (bFromSweep :type Boolean) (SweepResult :type Hit%20Result%20Structure%20%28by%20ref%29))
  (if (Variables|Default|GetIsActiviated)
    (Utilities|Casting|CastToBP_FirstPersonCharacter OtherActor)
    (Game|Feedback|ClientStartCameraShake (Game|GetPlayerController 0) "/Game/Blueprints/CameraShakes/BP_SphereActivatedShake.BP_SphereActivatedShake_C" 1.0 "CameraLocal" "0, 0, 0")))

(event OnComponentEndOverlap(Sphere1)
  (params (OverlappedComponent :type Primitive%20Component%20Object%20Reference) (OtherActor :type Actor%20Object%20Reference) (OtherComp :type Primitive%20Component%20Object%20Reference) (OtherBodyIndex :type Integer))
  (Utilities|Casting|CastToBP_FirstPersonCharacter OtherActor)
  (Game|Feedback|ClientStopCameraShake (Game|GetPlayerController 0) "/Game/Blueprints/CameraShakes/BP_SphereActivatedShake.BP_SphereActivatedShake_C" true))

(event Custom|OnActivated
  (bind _ground (Variables|Default|GetGround))
  (Development|PrintText "Hello")
  (Utilities|FlowControl|Delay 5.0)
  (Niagara|SpawnSystematLocation "/Game/ExtractionBeacon/NS_ExtractorBeam.NS_ExtractorBeam" (+ (Transformation|GetActorLocation) "0.000000,0.000000,490.000000") (Transformation|GetActorRotation))
  (Rendering|SetVisibility (Variables|Default|GetNS_ExtractionBeaconShockwave) false false)
  (Utilities|FlowControl|Delay 1.25)
  (Utilities|IsValid _ground
    (:Is%20Valid
      (Niagara|SetNiagaraVariable(Vector3) (Variables|/Script/Niagara.NiagaraActor|GetNiagaraComponent _ground) "GravityVector" "3.000000,0.000000,10.000000")
      (Sequencer|Player|Play (Variables|/Script/LevelSequence.LevelSequenceActor|GetSequencePlayer (Variables|Default|GetSequenceActor)) :!class /Script/MovieScene.MovieSceneSequencePlayer)
      (Utilities|FlowControl|Delay 1.0)
      (Variables|Default|SetMoveUp true)
      (Utilities|FlowControl|Delay 5.0)
      (bind _returnvalue (UserInterface|CreateWidget "/Game/Blueprints/Widgets/WB_End.WB_End_C"))
      (UserInterface|Viewport|AddtoViewport _returnvalue 0))))

(event Custom|SetLightning
  (Variables|Default|SetDoLightning true))

(event Custom|Transition
  (Game|OpenLevel(byName) "SecondScene"))

(event EventBeginPlay
  (bind _returnvalue (Rendering|Material|CreateDynamicMaterialInstance (Variables|Default|GetSphere2) 0 0 "None" :!class /Script/Engine.PrimitiveComponent))
  (Variables|Default|SetMaterialInstance _returnvalue)
  (if (Variables|Default|GetIsMainScene)
    (Variables|Default|SetDoLightning true)
    (bind _returnvalue_2 (Rendering|Material|CreateDynamicMaterialInstance (Variables|/Script/Engine.StaticMeshActor|GetStaticMeshComponent (Variables|Default|GetStaticMeshActor)) 0 0 "None" :!class /Script/Engine.PrimitiveComponent))
    (Variables|Default|SetNewVar _returnvalue_2)))

(event EventTick
  (params (DeltaSeconds :type Float%20%28single-precision%29))
  (bind _returnvalue (* DeltaSeconds 0.15))
  (Utilities|FlowControl|Sequence
    (:then_0
      (if (Variables|Default|GetIsActiviated)
        (Utilities|FlowControl|Sequence
          (:then_0
            (if (> (Variables|Default|GetTraceCooldown) (Variables|Default|GetMinCooldown))
              (Variables|Default|SetTraceCooldown (- (Variables|Default|GetTraceCooldown) DeltaSeconds))
              (else
                (Variables|Default|SetTraceCooldown (Variables|Default|GetMinCooldown)))))
          (:then_1
            (Rendering|Material|SetScalarParameterValue (Variables|Default|GetMaterialInstance) "TimeSpeed" (Math|Float|Lerp (Variables|Default|GetA) 1.0 _returnvalue) :!class /Script/Engine.MaterialInstanceDynamic)
            (Variables|Default|SetA (Math|Float|Lerp (Variables|Default|GetA) 1.0 _returnvalue))
            (Rendering|Components|Light|SetIntensity (Variables|Default|GetPointLight) (Math|Float|Lerp (Variables|Default|GetA_0) 2e+05 _returnvalue))
            (Variables|Default|SetA_0 (Math|Float|Lerp (Variables|Default|GetA_0) 2e+05 _returnvalue))
            (if (Variables|Default|GetMoveUp)
              (Variables|Default|SetTimeSinceStartedMoving (+ (Variables|Default|GetTimeSinceStartedMoving) DeltaSeconds))
              (Transformation|SetActorScale3D (Class|KismetMathLibrary|VectorSlerpNormals (Transformation|GetActorScale3D) "500.000000,500.000000,500.000000" DeltaSeconds))
              (Rendering|Material|SetScalarParameterValue "/Game/Materials/PostProcessing/MPC_ColorFill.MPC_ColorFill" "Intensity" (Math|Float|Lerp (Variables|Default|GetA_1) 1.0 (* DeltaSeconds 0.8)) :!class /Script/Engine.KismetMaterialLibrary)
              (Variables|Default|SetA_1 (Math|Float|Lerp (Variables|Default|GetA_1) 1.0 (* DeltaSeconds 0.8))))))))
    (:then_1
      (if (Variables|Default|GetDoLightning)
        (CallFunction|UpdateTraces)))))

(fn ConstructionScript)

(fn Interact
  (params (InActor :type Actor%20Object%20Reference))
  (if (Variables|Default|GetIsMainScene)
    (if (not (Variables|Default|GetIsActiviated))
      (if true
        (Variables|Default|SetIsActiviated true)
        (Variables|Default|SetDoLightning true)
        (Variables|Default|SetTraceCooldown (Variables|Default|GetMaxCoolDown))
        (Game|Feedback|ClientStartCameraShake (Game|GetPlayerController 0) "/Game/Blueprints/CameraShakes/BP_SphereActivatedShake.BP_SphereActivatedShake_C" 1.0 "CameraLocal" "0, 0, 0")
        (bind _outactors (Actor|GetAllActorsOfClass "/Game/Blueprints/BP_RockSpawner.BP_RockSpawner_C"))
        (CallFunction|OnActivated)
        (for _array_element _outactors
          (Default|SpawnRocks _array_element self))))
    (else
      (bind _returnvalue (Actor|GetActorOfClass "/Script/LevelSequence.LevelSequenceActor"))
      (Sequencer|Player|Play (Variables|/Script/LevelSequence.LevelSequenceActor|GetSequencePlayer _returnvalue) :!class /Script/MovieScene.MovieSceneSequencePlayer))))

(fn UpdateTraces
  (bind _returnvalue (Transformation|GetActorLocation))
  ;[1 1 1] TickCoolDown
  (if (>= (- (Utilities|Time|GetTimeSeconds) (Variables|Default|GetLastTrace)) (Variables|Default|GetTraceCooldown))
    (Variables|Default|SetLastTrace (Utilities|Time|GetTimeSeconds))
    (Variables|Default|SetRandomDir (Math|Random|RandomUnitVector))
    (bind _outhit (Collision|LineTraceByChannel (+ _returnvalue (* (Variables|Default|GetRandomDir) (Variables|Default|GetMinRadius))) (+ _returnvalue (* (Variables|Default|GetRandomDir) (Variables|Default|GetMaxRadius))) "TraceTypeQuery1" false 0 "None" true "(R=1.000000,G=0.000000,B=0.000000,A=1.000000)" "(R=0.000000,G=1.000000,B=0.000000,A=1.000000)" (Variables|Default|GetTraceCooldown)))
    (if (.bBlockingHit (Collision|BreakHitResult _outhit))
      (bind _returnvalue_2 (Niagara|SpawnSystemAttached "/Game/Particles/NS_LightniningBeam.NS_LightniningBeam" (Variables|Default|GetDefaultSceneRoot) "None" "0, 0, 0" "0, 0, 0" "KeepRelativeOffset" false))
      (Niagara|SetNiagaraVariable(Vector3) _returnvalue_2 "StartPos" (* (Variables|Default|GetRandomDir) (Variables|Default|GetMinRadius)))
      (Niagara|SetNiagaraVariable(Vector3) _returnvalue_2 "EndPos" (+ (.ImpactPoint (Collision|BreakHitResult _outhit)) (* (.ImpactNormal (Collision|BreakHitResult _outhit)) (LocalVariables|GetImpactOffset))))
      (Niagara|SetNiagaraVariable(Vector3) _returnvalue_2 "ImpactNormal" (.ImpactNormal (Collision|BreakHitResult _outhit))))))

(fn Pulse)

(fn UpdateWallVFX
  (bind _output_get (Variables|Default|SetMask (+ (Utilities|Time|GetWorldDeltaSeconds) (Variables|Default|GetMask))))
  (Rendering|Material|SetScalarParameterValue (Variables|Default|GetNewVar) "Mask" _output_get :!class /Script/Engine.MaterialInstanceDynamic))